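; Enemy AI character that chases and melee-attacks the player in a wave-based first-person game, with stats set through SetDefaults.
; FollowPlayer re-issues AIMoveTo on success, while AttackPlayer locks movement during an attack montage when in range.
; HitDetection sphere-traces at the right hand and applies damage, gated by the player's hit cooldown.
; Death ragdolls the mesh and decrements WaveGenerator_BP's enemy count, ending the wave at zero.
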(event `Set Defaults`
  (params (AttackDamage :type "Float (double-precision)") (AttackRange :type "Float (double-precision)") (WalkSpeed :type "Float (double-precision)") (AttackAnim :type "AnimMontage Object Reference") (SpawnValue :type Integer :default 1))
  ;[1 1 1] Set the default stats for this enemy (might be replaced with a better method later)
  (set `self.AttackDamage` AttackDamage)
  (set `self.AttackRange` AttackRange)
  (bind _output_get (set `self.WalkSpeed` WalkSpeed))
  (set `CharacterMovementComponent.MaxWalkSpeed` _output_get (`self.CharacterMovement`))
  (set `self.AttackAnim` AttackAnim)
  (set `self.SpawnValue` SpawnValue))

(event `Follow Player`
  ;[1 1 1] Always follow the player, unless currently attacking
  (if (`self.IsAlive`)
    (if (not (`self.IsAttacking`))
      (`CharacterMovementComponent.SetMovementMode` (`self.CharacterMovement`) "MOVE_Walking" 0)
      (`|AIMoveTo` self (0.0 0.0 0.0) (`GameplayStatics.GetPlayerCharacter` 0)
        (:`OnSuccess`
          (`self.Follow Player`))))))

(event `Attack Player`
  ;[1 1 1] If within range of the player, attempt to attack
  (if (`self.IsAlive`)
    (if (and (<= (`self.GetDistanceTo` (`GameplayStatics.GetPlayerCharacter` 0)) (`self.AttackRange`)) (!= (`self.IsAttacking`) true))
      (set `self.IsAttacking` true)
      (`CharacterMovementComponent.DisableMovement` (`self.CharacterMovement`))
      (`|PlayMontage` (`self.Mesh`) (`self.AttackAnim`)
        (:`OnCompleted`
          (`KismetSystemLibrary.Delay` 0.15))
        (:`OnInterrupted`
          _))
      (set `self.IsAttacking` false))))

(event `OnDeath`
  ;[1 1 1] When enemy dies
  (set `self.IsAlive` false)
  (`PrimitiveComponent.SetSimulatePhysics` (`self.Mesh`) true)
  (`ActorComponent.K2_DestroyComponent` (`self.CapsuleComponent`))
  (bind _returnvalue (`GameplayStatics.GetActorOfClass` "/Game/Blueprints/WaveGenerator_BP.WaveGenerator_BP_C"))
  (bind _output_get (set `/Game/Blueprints/WaveGenerator_BP.TotalEnemies` (- (`/Game/Blueprints/WaveGenerator_BP.TotalEnemies` _returnvalue) 1) _returnvalue))
  (if (== _output_get 0)
    (`KismetSystemLibrary.PrintString` "ENMIES GONE")
    (bind _returnvalue_2 (`GameplayStatics.GetActorOfClass` "/Game/Blueprints/WaveGenerator_BP.WaveGenerator_BP_C"))
    (`/Game/Blueprints/WaveGenerator_BP.OnWaveEnd` _returnvalue_2)))

(event `self.ReceiveAnyDamage`
  (params (Damage :type "Float (single-precision)") (DamageType :type "DamageType Object Reference") (InstigatedBy :type "Controller Object Reference") (DamageCauser :type "Actor Object Reference"))
  ;[1 1 1] When enemy takes damage
  (bind _output_get (set `self.Health` (- (`self.Health`) Damage)))
  (if (<= _output_get 0.0)
    (`self.OnDeath`)))

(fn `HitDetection`
  (bind _returnvalue (`SceneComponent.GetSocketLocation` (`self.Mesh`) "RightHand"))
  (bind _outhit (`KismetSystemLibrary.SphereTraceSingleForObjects` _returnvalue _returnvalue 90.0 (`|MakeArray` "ObjectTypeQuery2" :!type "EObjectTypeQuery Enum")))
  (bind _asbp_first_person_character (cast `/Game/FirstPerson/Blueprints/BP_FirstPersonCharacter` (`.HitActor` (`GameplayStatics.BreakHitResult` _outhit))))
  (if (>= (`/Game/FirstPerson/Blueprints/BP_FirstPersonCharacter.TimeSinceLastHit` _asbp_first_person_character) (`/Game/FirstPerson/Blueprints/BP_FirstPersonCharacter.TimeBetweenHits` _asbp_first_person_character))
    (`GameplayStatics.ApplyDamage` (`GameplayStatics.GetPlayerCharacter` 0) (`self.AttackDamage`))
    (bind _asbp_first_person_character_2 (cast `/Game/FirstPerson/Blueprints/BP_FirstPersonCharacter` (`GameplayStatics.GetPlayerCharacter` 0)))
    (set `/Game/FirstPerson/Blueprints/BP_FirstPersonCharacter.TimeSinceLastHit` 0.0 _asbp_first_person_character_2)
    (`KismetSystemLibrary.PrintString` (`KismetStringLibrary.Conv_DoubleToString` (`/Game/FirstPerson/Blueprints/BP_FirstPersonCharacter.Health` _asbp_first_person_character_2)))))

(fn `IncementHitCooldown`
  (set `self.TimeSinceLastHit` (+ (`self.TimeSinceLastHit`) (`GameplayStatics.GetWorldDeltaSeconds`))))

(fn `UserConstructionScript`)