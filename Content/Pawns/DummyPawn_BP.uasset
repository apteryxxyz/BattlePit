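; DummyPawn_BP is a simple damageable dummy pawn that loses health when hit and destroys itself once health runs out.
; Tick accumulates the time since the last hit.
; The Hit function resets that timer, decrements Health by one, then either destroys the actor or prints the remaining health.
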(event `self.ReceiveTick`
  (params (DeltaSeconds :type "Float (single-precision)"))
  ;[1 1 1] Increment TimeSinceLastHit with time
  (set `self.TimeSinceLatHit` (+ (`self.TimeSinceLatHit`) DeltaSeconds)))

(fn `Hit`
  (set `self.TimeSinceLatHit` 0.0)
  (bind _result (`/Engine/EditorBlueprintResources/StandardMacros.DecrementInt` (`self.Health`))
    (:`  `
      (set `self.Health` _result)
      (if (<= (`self.Health`) 0)
        (`self.K2_DestroyActor`)
        (else
          (`KismetSystemLibrary.PrintString` (`KismetStringLibrary.Conv_IntToString` (`self.Health`))))))))

(fn `UserConstructionScript`)