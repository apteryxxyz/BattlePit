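; CaptainBanner_BP is a banner actor that scales the attack damage of BP_EnemyAI actors while they overlap it.
; Begin overlap multiplies the enemy's AttackDamage by StatMultipler, and end overlap sets it to the stored DefaultDamage.
; A single Enemy reference and DefaultDamage serve all enemies.
; SetDefaultStats captures damage before Enemy is reassigned, so it reads the previously referenced enemy.
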(event `self.ReceiveActorBeginOverlap`
  (params (OtherActor :type "Actor Object Reference"))
  (`self.SetDefaultStats`)
  (bind _asbp_enemy_ai (cast `/Game/EnemyAI/BP_EnemyAI` OtherActor))
  (set `self.enemy` _asbp_enemy_ai)
  (set `/Game/EnemyAI/BP_EnemyAI.AttackDamage` (* (`/Game/EnemyAI/BP_EnemyAI.AttackDamage` (`self.enemy`)) (`self.statMultipler`)) (`self.enemy`)))

(event `self.ReceiveActorEndOverlap`
  (params (OtherActor :type "Actor Object Reference"))
  (bind _asbp_enemy_ai (cast `/Game/EnemyAI/BP_EnemyAI` OtherActor))
  (set `self.enemy` _asbp_enemy_ai)
  (set `/Game/EnemyAI/BP_EnemyAI.AttackDamage` (`self.defaultDamage`) (`self.enemy`)))

(event `SetDefaultStats`
  (set `self.defaultDamage` (`/Game/EnemyAI/BP_EnemyAI.AttackDamage` (`self.enemy`))))

(fn `UserConstructionScript`)