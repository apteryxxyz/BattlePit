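; WaveGenerator_BP runs enemy waves, starting one on BeginPlay and another after a cooldown whenever OnWaveEnd fires.
; Each wave passes WaveValue to every EnemySpawner_BP found in the level, then increments WaveNumber.
; WaveValue grows exponentially with the wave number from an initial value and multiplier.
; It is recalculated on Tick and before each follow-up wave; the Delay after the Tick update gates nothing.
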(event `self.ReceiveTick`
  (params (DeltaSeconds :type "Float (single-precision)"))
  (`self.AdjustWaveDifficulty`)
  (`KismetSystemLibrary.Delay` 0.35))

(event `self.ReceiveBeginPlay`
  (`self.GenerateWave`))

(event `OnWaveEnd`
  (`KismetSystemLibrary.Delay` (`self.WaveCooldown`))
  (`self.AdjustWaveDifficulty`)
  (set `self.SpawnedValue` 0)
  (`self.GenerateWave`))

(event `GenerateWave`
  (bind _outactors (`GameplayStatics.GetAllActorsOfClass` "/Game/Blueprints/EnemySpawner_BP.EnemySpawner_BP_C"))
  (for _array_element _outactors
    (`/Game/Blueprints/EnemySpawner_BP.SpawnEnemies` _array_element (`self.WaveValue`) 2.0))
  (set `self.WaveNumber` (+ (`self.WaveNumber`) 1)))

(event `AdjustWaveDifficulty`
  (set `self.WaveValue` (+ (`KismetMathLibrary.FTrunc` (* (`self.InitialWaveValue`) (`KismetMathLibrary.Exp` (`KismetMathLibrary.Conv_IntToDouble` (* (`self.WaveNumber`) (`self.WaveValueMultiplier`)))))) 1)))

(fn `UserConstructionScript`)