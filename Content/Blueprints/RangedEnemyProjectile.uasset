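; Projectile for a ranged enemy that launches itself at player 0 and damages them on contact.
; On BeginPlay it leads the target by player velocity times distance over ProjectileSpeed, then solves a toss velocity with SuggestProjectileVelocity.
; That velocity drives ProjectileMovement, with rotation following the flight path.
; Overlapping BP_FirstPersonCharacter applies AIOwner's AttackDamage to player 0, without destroying the projectile in this graph.
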(event `self.ReceiveBeginPlay`
  (bind _returnvalue (`GameplayStatics.GetPlayerCharacter` 0))
  (bind _projectilemovement (`self.ProjectileMovement`))
  (bind _tossvelocity (`GameplayStatics.BlueprintSuggestProjectileVelocity` (`self.K2_GetActorLocation`) (+ (`self.K2_GetActorLocation` _returnvalue) (* (/ (`self.GetDistanceTo` _returnvalue) (`self.ProjectileSpeed`)) (`self.GetVelocity` _returnvalue))) (`self.ProjectileSpeed`) 0.0 "DoNotTrace"))
  (set `MovementComponent.Velocity` _tossvelocity _projectilemovement)
  (set `ProjectileMovementComponent.bRotationFollowsVelocity` true _projectilemovement))

(event `self.ReceiveActorBeginOverlap`
  (params (OtherActor :type "Actor Object Reference"))
  (cast `/Game/FirstPerson/Blueprints/BP_FirstPersonCharacter` OtherActor)
  (`GameplayStatics.ApplyDamage` (`GameplayStatics.GetPlayerCharacter` 0) (`/Game/EnemyAI/BP_EnemyAI.AttackDamage` (`self.AIOwner`))))

(fn `UserConstructionScript`)