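; BP_EnemyAI is an enemy character base that chases the first player and deals melee-range damage.
; SetDefaults stores damage, range and walk speed, and applies the speed to CharacterMovement.
; FollowPlayer issues AI MoveTo unless attacking and calls itself again only on success.
; AttackPlayer applies damage directly when in range, a placeholder for animated hit detection, with IsAttacking and a delay serving as cooldown.
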(event `Set Defaults`
  (params (AttackDamage :type "Float (double-precision)") (AttackRange :type "Float (double-precision)") (WalkSpeed :type "Float (double-precision)"))
  ;[1 1 1] Set the default stats for this enemy (might be replaced with a better method later)
  (set `self.AttackDamage` AttackDamage)
  (set `self.AttackRange` AttackRange)
  (bind _output_get (set `self.WalkSpeed` WalkSpeed))
  (set `CharacterMovementComponent.MaxWalkSpeed` _output_get (`self.CharacterMovement`)))

(event `Follow Player`
  ;[1 1 1] Always follow the player, unless currently attacking
  (if (not (`self.IsAttacking`))
    (`|AIMoveTo` self (0.0 0.0 0.0) (`GameplayStatics.GetPlayerCharacter` 0)
      (:`OnSuccess`
        (`self.Follow Player`)))))

(event `Attack Player`
  ;[1 1 1] If within range of the player, attempt to attack
  (if (and (<= (`self.GetDistanceTo` (`GameplayStatics.GetPlayerCharacter` 0)) (`self.AttackRange`)) (!= (`self.IsAttacking`) true))
    (set `self.IsAttacking` true)
    ;;[1 1 1 1 12] This should be replaced with an animation plus hit detection on the enemies weapon
    (`GameplayStatics.ApplyDamage` (`GameplayStatics.GetPlayerCharacter` 0) (`self.AttackDamage`))
    (`KismetSystemLibrary.Delay` 2.0)
    (set `self.IsAttacking` false)))

(fn `UserConstructionScript`)